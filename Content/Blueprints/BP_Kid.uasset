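; BP_Kid is a keyboard-controlled pawn that moves back and forth along the world X axis.
; W and S key events set held-state booleans, which Tick reads to add forward or backward movement input, with W taking priority.
; Movement uses fixed world directions, and two Y-axis movement nodes are left unconnected, so sideways movement is inactive.
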(event `self.ReceiveTick`
  (params (DeltaSeconds :type "Float (single-precision)"))
  (if (`self.W_Down`)
    (`self.AddMovementInput` (1.0 0.0 0.0))
    (elif (`self.S_Down`)
      (`self.AddMovementInput` (1.0 0.0 0.0) -1.0))))

(event `Key|W`
  (params (Key :type "Key Structure"))
  (:`Pressed`
    (set `self.W_Down` true))
  (:`Released`
    (set `self.W_Down` false)))

(event `Key|S`
  (params (Key :type "Key Structure"))
  (:`Pressed`
    (set `self.S_Down` true))
  (:`Released`
    (set `self.S_Down` false)))

(event `Key|A`
  (params (Key :type "Key Structure")))

(event `Key|D`
  (params (Key :type "Key Structure")))

(fn `UserConstructionScript`)