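; BP_Gun is a gun Blueprint with pickup-prompt logic driven by overlaps on its Collider.
; Any actor beginning an overlap creates a new WBP_PickUp_UI widget, stores it in PickUpUi and adds it to the viewport.
; For the player character only, it also calls StartTraceMessage on that character, passing false on entry and true on exit.
; The widget is created before the player check and is not removed in this graph.
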(event `self.Collider.OnComponentBeginOverlap`
  (params (OverlappedComponent :type "PrimitiveComponent Object Reference") (OtherActor :type "Actor Object Reference") (OtherComp :type "PrimitiveComponent Object Reference") (OtherBodyIndex :type Integer) (bFromSweep :type Boolean) (SweepResult :type "HitResult Structure (by ref)"))
  (bind _returnvalue (`GameplayStatics.GetPlayerCharacter` 0))
  (if true
    (bind _returnvalue_2 (`|CreateWidget` "/Game/Guts_Game/UI/WBP_PickUp_UI.WBP_PickUp_UI_C"))
    (bind _output_get (set `self.Pick up ui` _returnvalue_2))
    (`UserWidget.AddToViewport` _output_get 0)
    (if (== OtherActor _returnvalue)
      (message `/Game/Guts_Game/BluePrints/CharBPInterface.Start trace` _returnvalue false))))

(event `self.Collider.OnComponentEndOverlap`
  (params (OverlappedComponent :type "PrimitiveComponent Object Reference") (OtherActor :type "Actor Object Reference") (OtherComp :type "PrimitiveComponent Object Reference") (OtherBodyIndex :type Integer))
  (bind _returnvalue (`GameplayStatics.GetPlayerCharacter` 0))
  (if (== OtherActor _returnvalue)
    (message `/Game/Guts_Game/BluePrints/CharBPInterface.Start trace` _returnvalue true)))

(fn `UserConstructionScript`)