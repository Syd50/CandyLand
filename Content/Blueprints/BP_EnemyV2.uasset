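; Enemy character that damages actors leaving its collider sphere, can be staggered by throwables, and ends the game on death.
; AnyDamage sets Health to damage minus Health; at zero or below it plays a death animation and stops the AI's StateTree.
; After a delay it plays the kid-win sequence, then swaps gameplay UI for the main menu.
; Throwable halves walk speed, with a timer by function name to restore it.
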(event `self.ReceiveBeginPlay`
  ; Enemy walk speed after item is being thrown
  (set `self.Default walk speed` (`CharacterMovementComponent.MaxWalkSpeed` (`self.CharacterMovement`))))

(event `self.ReceiveAnyDamage`
  (params (Damage :type "Float (single-precision)") (DamageType :type "DamageType Object Reference") (InstigatedBy :type "Controller Object Reference") (DamageCauser :type "Actor Object Reference"))
  ; If shot 3 times destroy actor
  (if (not (`self.IsDead`))
    (bind _output_get (set `self.Health` (- Damage (`self.Health`))))
    (if (<= _output_get 0.0)
      (set `self.IsDead` true)
      (`SkeletalMeshComponent.PlayAnimation` (`self.Mesh`) "/Game/Mascot3/Animations/AS_Mascot3_Death2.AS_Mascot3_Death2" false)
      (bind _asaic_enemy (cast `/Game/Blueprints/StateTrees/AIC_Enemy` (`self.GetController`)))
      (`BrainComponent.StopLogic` (`/Game/Blueprints/StateTrees/AIC_Enemy.StateTreeAI` _asaic_enemy) "")
      (`KismetSystemLibrary.Delay` 8.0)
      (bind (_outactor _returnvalue) (`LevelSequencePlayer.CreateLevelSequencePlayer` "/Game/CINEMATICS/SQ_Kid_Win.SQ_Kid_Win"))
      (`MovieSceneSequencePlayer.Play` _returnvalue)
      (add `MovieSceneSequencePlayer.OnFinished` _returnvalue (delegate `OnDeathFinished`)))))

(event `OnDeathFinished`
  (bind _returnvalue (`GameplayStatics.GetPlayerController` 0))
  ; If shot 3 times destroy actor
  (bind _returnvalue_2 (`|CreateWidget` "/Game/Guts_Game/UI/WBP_MainMenu.WBP_MainMenu_C"))
  (`UserWidget.AddToViewport` _returnvalue_2 0)
  (set `PlayerController.bShowMouseCursor` true _returnvalue)
  (`WidgetBlueprintLibrary.SetInputMode_UIOnlyEx` _returnvalue _returnvalue_2)
  (bind _foundwidgets (`WidgetBlueprintLibrary.GetAllWidgetsOfClass` "/Game/Guts_Game/UI/WBP_GameplayUI.WBP_GameplayUI_C"))
  (for _array_element _foundwidgets
    (`Widget.RemoveFromParent` _array_element)))

(event `self.Sphere_collider.OnComponentEndOverlap`
  (params (OverlappedComponent :type "PrimitiveComponent Object Reference") (OtherActor :type "Actor Object Reference") (OtherComp :type "PrimitiveComponent Object Reference") (OtherBodyIndex :type Integer))
  ; If enemy collides with player damage them
  (if (not (`self.IsDead`))
    (`GameplayStatics.ApplyDamage` OtherActor 25.0 null self)))

(fn `Reset walk speed`
  (set `CharacterMovementComponent.MaxWalkSpeed` (`self.Default walk speed`) (`self.CharacterMovement`)))

(fn `Throwable`
  (returns (Return :type Boolean))
  (set `CharacterMovementComponent.MaxWalkSpeed` (/ (`self.Default walk speed`) 2.0) (`self.CharacterMovement`))
  (`KismetSystemLibrary.K2_SetTimer` null "Reset walk speed" (`self.StaggerDuration`))
  (return false))

(fn `UserConstructionScript`)